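; MiniGameGM is the mini-game's game mode, which tracks player controllers and handles their respawns.
; When a player restarts, it records the controller and, for a GameplayPC, caches all PlayerStart actors as respawn points and calls MiniGameSetup on that controller.
; The respawn2 event destroys the controller's current pawn, then spawns a 0_Base at a random cached point and possesses it.
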(event `self.K2_OnRestartPlayer`
  (params (NewPlayer :type "Controller Object Reference"))
  (bind _asplayer_controller (cast `PlayerController` NewPlayer :!pure true))
  (`KismetArrayLibrary.Array_Add` (`self.AllPlayersControllers`) _asplayer_controller)
  (bind _asgameplay_pc (cast `/Game/Blueprints/Gameplay/GameplayPC` _asplayer_controller))
  (bind _outactors (`GameplayStatics.GetAllActorsOfClass` "/Script/Engine.PlayerStart"))
  (set `self.RespawnPoints` _outactors)
  (`/Game/Blueprints/Gameplay/GameplayPC.MiniGameSetup` _asgameplay_pc))

(event `respawn 2`
  (params (`Player Controller` :type "PlayerController Object Reference"))
  (bind _returnvalue (`Controller.K2_GetPawn` `Player Controller`))
  (bind _respawnpoints (`self.RespawnPoints`))
  (`/Engine/EditorBlueprintResources/StandardMacros.IsValid` _returnvalue
    (:`Is Valid`
      (`self.K2_DestroyActor` _returnvalue))
    (:`Is Not Valid`
      _))
  (bind _returnvalue_2 (`|SpawnActorFromClass` "/Game/Blueprints/Characters/0_Base.0_Base_C" (`self.GetTransform` (`|GetArrayItem` _respawnpoints (`KismetMathLibrary.RandomInteger` (`KismetArrayLibrary.Array_Length` _respawnpoints)))) "Undefined" "OverrideRootScale" null null))
  (`Controller.Possess` `Player Controller` _returnvalue_2))

(fn `UserConstructionScript`)