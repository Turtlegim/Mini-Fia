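; Player controller for a multiplayer game with jobs, missions, chat, player voting and minigames, linking each player's UI to the game modes.
; It loads the saved name and image, requests spawning, and builds the HUD, vote, score and loading widgets.
; Chat fans out to all controllers, and votes go to GameplayGM, with a random fallback for missed votes.
; A six-slot DataTable-driven inventory uses number keys, with only the searching item acting, revealing another player's items.
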(event `PlayStart`
  (params (playerinfo :type "/Game/Blueprints/AllLevels/PlayerInfo Structure"))
  ;[1 1 1] 플레이어 정보를 가져와 서버에게 넘겨줌
  (set `self.Player Setting` playerinfo)
  (`WidgetLayoutLibrary.RemoveAllWidgets`)
  (`self.LoadGame`)
  (`self.ControllerPassServer` (`self.Player Setting`)))

(event `Mini1_updatescore`
  (params (NewParam :type "Array of Integer (by ref)"))
  (bind _returnvalue (`|CreateWidget` "/Game/UI/MiniGame_Climb/Score_UI.Score_UI_C" self))
  (`/Game/UI/MiniGame_Climb/Score_UI.UpdateScore` _returnvalue NewParam (`self.All Player Info`))
  (`UserWidget.AddToViewport` _returnvalue 0))

(event `ControllerPassServer`
  (params (PlayerSetting :type "/Game/Blueprints/AllLevels/PlayerInfo Structure"))
  ;[1 1 1] 플레이어 세팅상태로 스폰
  (set `self.Player Setting` PlayerSetting)
  (bind _asgameplay_gm (cast `/Game/Blueprints/Gameplay/GameplayGM` (`GameplayStatics.GetGameMode`)))
  (`/Game/Blueprints/Gameplay/GameplayGM.RespawnPlayer` _asgameplay_gm self)
  (`self.SetUpChatWindow`)
  (`/Game/Blueprints/Gameplay/GameplayGM.CheckAllSpawn2` _asgameplay_gm))

(event `MiniGameSetup`
  (bind _asmini_game_gm (cast `/Game/Blueprints/MiniGame/MiniGameGM` (`GameplayStatics.GetGameMode`)))
  (`/Game/Blueprints/MiniGame/MiniGameGM.respawn 2` _asmini_game_gm self)
  (`self.MinigameWind`)
  (`self.SetUpChatWindow`))

(event `MIni1_clear`
  (`PanelWidget.ClearChildren` (`/Game/UI/MiniGame_Climb/Score_UI.VerticalBox_154` (stale `Mini1_updatescore` _returnvalue))))

(event `SetUpChatWindow`
  ;[1 1 1] 채팅 창 생성 후 뷰포트 추가
  (bind _returnvalue (`|CreateWidget` "/Game/UI/AllLevels/GameplayChat.GameplayChat_C"))
  (bind _output_get (set `self.GamePlayChat WB` _returnvalue))
  (`UserWidget.AddToViewport` _output_get 0)
  (`WidgetBlueprintLibrary.SetInputMode_GameOnly` self))

(event `MinigameWind`
  (`WidgetLayoutLibrary.RemoveAllWidgets`))

(event `ShowLoadingScreen`
  (`WidgetLayoutLibrary.RemoveAllWidgets`)
  (bind _returnvalue (`|CreateWidget` "/Game/UI/AllLevels/LoadingScreen.LoadingScreen_C" self))
  (`UserWidget.AddToViewport` _returnvalue 0))

(event `GetChat`
  (params (`Text to Send` :type Text))
  ;[1 1 1] 입력된 채팅을 처리하고 각 플레이어에게 업데이트하라고 통보
  (set `self.Text` `Text to Send`)
  (set `self.Sender` (`.MyPlayerName_2_0D47280F4CABE4536CA4C0A701BBEDF7` (break `/Game/Blueprints/AllLevels/PlayerInfo` (`self.Player Setting`))))
  (bind _asgameplay_gm (cast `/Game/Blueprints/Gameplay/GameplayGM` (`GameplayStatics.GetGameMode`)))
  (for _array_element (`/Game/Blueprints/Gameplay/GameplayGM.AllPlayerControllers` _asgameplay_gm)
    (bind _asgameplay_pc (cast `/Game/Blueprints/Gameplay/GameplayPC` _array_element))
    (`self.UpdateChat` _asgameplay_pc (`self.Text`) (`self.Sender`) (struct :`R` 1.0 :`G` 1.0 :`B` 1.0 :`A` 1.0))))

(event `MouseTrueMoveStop`
  ;[1 1 1] 마우스 커서가 있으면 동작 중지
  (if (`self.bShowMouseCursor`)
    (bind _as0_base (cast `/Game/Blueprints/Characters/0_Base` (`GameplayStatics.GetPlayerCharacter` 0)))
    (set `/Game/Blueprints/Characters/0_Base.isMouse` true _as0_base)
    (else
      (set `/Game/Blueprints/Characters/0_Base.isMouse` false _as0_base))))

(event `MIniGameWinnerNoti`
  (params (winner :type Text))
  (bind _returnvalue (`|CreateWidget` "/Game/UI/PlayerStatus/MiniGameWinner.MiniGameWinner_C" self winner))
  (`UserWidget.AddToViewport` _returnvalue 0))

(event `DestroyLoadingScreen`
  (if (`Widget.IsInViewport` (stale `ShowLoadingScreen` _returnvalue))
    (`Widget.RemoveFromParent` (stale `ShowLoadingScreen` _returnvalue))))

(event `GetRandItem`
  (bind _asmini_game_gm (cast `/Game/Blueprints/MiniGame/MiniGameGM` (`GameplayStatics.GetGameMode`)))
  (`/Game/Blueprints/MiniGame/MiniGameGM.MakeRandomItem` _asmini_game_gm)
  (`KismetSystemLibrary.Delay` 0.2)
  (`self.SendItemToClient` (`/Game/Blueprints/MiniGame/MiniGameGM.ItemArray` _asmini_game_gm)))

(event `UpdateChat`
  (params (Text :type Text) (Sender :type Text) (ChatColor :type "LinearColor Structure"))
  ;[1 1 1] 채팅창 업데이트
  (`/Game/UI/AllLevels/ChatWindow.UpdateChatWindow` (`/Game/UI/AllLevels/GameplayChat.GamePlayerChat` (`self.GamePlayChat WB`)) Sender Text ChatColor))

(event `Key|T`
  (params (Key :type "Key Structure"))
  ;[1 1 1] T키를 누르면 마우스 커서 토글
  (:`Pressed`
    (`/Engine/EditorBlueprintResources/StandardMacros.FlipFlop`
      (:`A`
        (set `self.bShowMouseCursor` true))
      (:`B`
        (set `self.bShowMouseCursor` false)))
    (`self.MouseTrueMoveStop`)))

(event `Key|C`
  (params (Key :type "Key Structure"))
  (bind _gameplayerchat (`/Game/UI/AllLevels/GameplayChat.GamePlayerChat` (`self.GamePlayChat WB`)))
  ;[1 1 1] C키를 누르면 채팅창 토글
  (:`Pressed`
    (if (`Widget.IsVisible` _gameplayerchat)
      (`Widget.SetVisibility` _gameplayerchat "Collapsed")
      (else
        (`Widget.SetVisibility` _gameplayerchat "Visible")))))

(event `Key|M`
  (params (Key :type "Key Structure"))
  (bind _missioonwindow (`/Game/UI/AllLevels/JobAndInfo.MissioonWindow` (`/Game/UI/AllLevels/GameplayChat.JobAndInfo` (`self.GamePlayChat WB`))))
  ;[1 1 1] M키를 누르면 미션창 크기 변화
  (:`Pressed`
    (if (`ExpandableArea.GetIsExpanded` _missioonwindow)
      (`ExpandableArea.SetIsExpanded` _missioonwindow false)
      (else
        (`ExpandableArea.SetIsExpanded` _missioonwindow true)))))

(event `Key|I`
  (params (Key :type "Key Structure")))

(event `UpdateMission`
  ;[1 1 1] 미션 창 업데이트
  (`/Game/UI/AllLevels/JobAndInfo.UpdateMission` (`/Game/UI/AllLevels/GameplayChat.JobAndInfo` (`self.GamePlayChat WB`))))

(event `UpdateJob`
  ;[1 1 1] 직업 창 업데이트
  (`/Game/UI/AllLevels/JobAndInfo.UpdateJob` (`/Game/UI/AllLevels/GameplayChat.JobAndInfo` (`self.GamePlayChat WB`))))

(event `SendItemToClient`
  (params (Item :type "Array of /Game/Blueprints/AllLevels/ItemData Structure"))
  (bind _returnvalue (`|CreateWidget` "/Game/UI/PlayerStatus/SelectItem.SelectItem_C" self Item))
  (`/Game/UI/PlayerStatus/SelectItem.Make3Item` _returnvalue)
  (`UserWidget.AddToViewport` _returnvalue 0))

(event `Key|Enter`
  (params (Key :type "Key Structure"))
  ;[1 1 1] 엔터를 누르면 채팅 가능
  (:`Pressed`
    (`/Game/UI/AllLevels/GameplayChat.ChatSystemUse` (`self.GamePlayChat WB`))))

(event `AddItemList`
  (bind _gameplaychat_wb (`self.GamePlayChat WB`))
  ;[1 1 1] 호출하면 위젯에 소유 아이템 업데이트
  (`/Engine/EditorBlueprintResources/StandardMacros.IsValid` _gameplaychat_wb
    (:`Is Valid`
      (`/Game/UI/AllLevels/GameplayChat.ClearInven` _gameplaychat_wb)
      (`/Game/UI/AllLevels/GameplayChat.UpdateInven` _gameplaychat_wb (`self.Inventory`)))))

(event `Server_multi_unposses`
  ;[1 1 1] Unposses
  (`self.UnPossess`))

(event `Key|O`
  (params (Key :type "Key Structure"))
  (:`Pressed`
    (`self. Get item` "bulletproof")))

(event `Key|P`
  (params (Key :type "Key Structure"))
  (:`Pressed`
    (`self. Get item` "gun")))

(event `Test to death`
  ;[1 1 1] 플레이어 사망
  (`WidgetLayoutLibrary.RemoveAllWidgets`)
  (bind _returnvalue (`|CreateWidget` "/Game/UI/AllLevels/VoteSetting/Test.Test_C"))
  (`UserWidget.AddToViewport` _returnvalue 0)
  (`self.GetChat` "가 사망했습니다")
  (`KismetSystemLibrary.Delay` 2.0)
  (`self.Server_multi_unposses`))

(event `Key|L`
  (params (Key :type "Key Structure"))
  (:`Pressed`
    (`self. Get item` "searching")))

(event `UpdateTimer`
  (params (RemainingTime :type "Float (double-precision)"))
  (bind _timer (`/Game/UI/AllLevels/VoteSetting/RemainTime.Timer` (`/Game/UI/AllLevels/GameplayChat.remaintime` (`self.GamePlayChat WB`))))
  ;[1 1 1] 1초마다 시간 업데이트
  (set `/Game/UI/AllLevels/VoteSetting/Timer.Sec` RemainingTime _timer)
  (`/Game/UI/AllLevels/VoteSetting/Timer.Timer` _timer))

(event `UpdateTimer2`
  (params (Sec2 :type "Float (double-precision)"))
  ;[1 1 1] 1초마다 시간 업데이트
  (`/Game/UI/AllLevels/VoteSetting/VoteWidget.GetVoteRemainingTime` (`self.Vote WB`) Sec2))

(event `Key|V`
  (params (Key :type "Key Structure"))
  (:`Pressed`
    (bind _asgameplay_gm (cast `/Game/Blueprints/Gameplay/GameplayGM` (`GameplayStatics.GetGameMode`)))
    (`/Game/Blueprints/Gameplay/GameplayGM.MiniGame` _asgameplay_gm)))

(event `Makevotewindow`
  (params (`All info` :type "Array of /Game/Blueprints/AllLevels/PlayerInfo Structure"))
  ;[1 1 1] 투표창 위젯을 생성
  (set `self.bShowMouseCursor` true)
  (set `self.Has_Widget` true)
  (`self.MouseTrueMoveStop`)
  (set `self.All Player Info` `All info`)
  (bind _returnvalue (`|CreateWidget` "/Game/UI/AllLevels/VoteSetting/VoteWidget.VoteWidget_C"))
  (set `self.Vote WB` _returnvalue)
  (for _array_element (`self.All Player Info`)
    (`/Game/UI/AllLevels/VoteSetting/VoteWidget.PlayerSetting` (`self.Vote WB`) _array_element))
  (`UserWidget.AddToViewport` (`self.Vote WB`) 0))

(event `GetVotePlayerIndex`
  (params (Index :type Integer) (Voted :type Boolean))
  ;[1 1 1] 투표 창에서 투표한 플레이어의 인덱스를 받아와 게임모드에 저장(투표 시간이 지나 투표를 못했으면 랜덤으로 투표)
  (set `self.VotePlayerIndex` Index)
  (set `self.Voted` Voted)
  (bind _asgameplay_gm (cast `/Game/Blueprints/Gameplay/GameplayGM` (`GameplayStatics.GetGameMode`)))
  (if (== (`self.VotePlayerIndex`) -1)
    (set `self.VotePlayerIndex` (`KismetMathLibrary.RandomInteger` (`KismetArrayLibrary.Array_Length` (`/Game/Blueprints/Gameplay/GameplayGM.PlayerVote` _asgameplay_gm)))))
  (`/Engine/EditorBlueprintResources/StandardMacros.IncrementInt` (`|GetArrayItem` (`/Game/Blueprints/Gameplay/GameplayGM.PlayerVote` _asgameplay_gm) (`self.VotePlayerIndex`))
    (:`  `
      (`/Game/Blueprints/Gameplay/GameplayGM.CheckVoteComplete` _asgameplay_gm))))

(event `InformPickedPlayer`
  (params (`Picked Player Info` :type "/Game/Blueprints/AllLevels/PlayerInfo Structure"))
  (bind (_myplayername _myplayerimage _myplayerjob) (break `/Game/Blueprints/AllLevels/PlayerInfo` `Picked Player Info`))
  ;[1 1 1] 투표결과를 받아와 위젯에 띄움
  (`/Game/UI/AllLevels/VoteSetting/VoteWidget.PrintVoteResult` (`self.Vote WB`) _myplayername _myplayerjob)
  (set `self.Has_Widget` false)
  (set `self.bShowMouseCursor` false)
  (`WidgetBlueprintLibrary.SetInputMode_GameOnly` self)
  (`self.MouseTrueMoveStop`))

(event `ReadyRevote`
  (params (RevotePlayer :type "Array of /Game/Blueprints/AllLevels/PlayerInfo Structure"))
  ;[1 1 1] 재투표 준비를 하고 동일한 투표 수가 나온 것을 알림
  (`/Game/UI/AllLevels/VoteSetting/VoteWidget.NoticeRevote` (`self.Vote WB`))
  (`KismetSystemLibrary.Delay` 2.0)
  (`self.Makevotewindow` RevotePlayer))

(event `Get item`
  (params (NewParam :type Text))
  ;[1 1 1] 아이템 획득을 업데이트하고 위젯에 알림
  (if (not (> (`KismetArrayLibrary.Array_Length` (`self.Inventory`)) 5))
    (bind _returnvalue (`|GetDataTableRow` "/Game/Blueprints/AllLevels/itemdatatable.itemdatatable" (`KismetStringLibrary.Conv_StringToName` (`KismetTextLibrary.Conv_TextToString` NewParam)))
      (:`then`
        (`KismetArrayLibrary.Array_Add` (`self.Inventory`) _returnvalue)
        (`self.AddItemList`)
        (`self.Get Item To Server` (`self.Inventory`))))))

(event `Get Item To Server`
  (params (S_inven :type "Array of /Game/Blueprints/AllLevels/ItemData Structure"))
  ;[1 1 1] 아이템 획득을 업데이트하고 위젯에 알림
  (set `self.Inventory` S_inven))

(event `Key|One`
  (params (Key :type "Key Structure"))
  ;[1 1 1] 아이템 사용 키 바인드
  (:`Pressed`
    (`self.UseItemSelect` 1)))

(event `UseItemSelect`
  (params (PushNum :type Integer))
  (bind _returnvalue (- PushNum 1))
  (bind _inventory (`self.Inventory`))
  ;[1 1 1] 인벤이 열려있을 때 숫자키 (1-6)을 누르면 그 인덱스에 맞는 아이템 사용
  (if (`Widget.IsInViewport` (stale `Key|E` _returnvalue))
    (if (`KismetArrayLibrary.Array_IsValidIndex` _inventory _returnvalue)
      (bind _itemtableindex (`self.Ckeck Item` (`|GetArrayItem` _inventory _returnvalue)))
      (if (== _itemtableindex 1)
        _
        (elif (== _itemtableindex 2)
          _
          (elif (== _itemtableindex 3)
            (`self.Use Item(Searching)`))))
      (else
        (`self.UpdateChat` (`|FormatText` "{a}번째 아이템이 없습니다." PushNum) "[Sysyem]" (struct :`R` 0.712 :`G` 0.03108 :`A` 1.0))))))

(event `Key|E`
  (params (Key :type "Key Structure"))
  ;[1 1 1] E키를 입력시 인벤 활성화 및 아이템 사용가능
  (:`Pressed`
    (`/Engine/EditorBlueprintResources/StandardMacros.FlipFlop`
      (:`A`
        (bind _returnvalue (`|CreateWidget` "/Game/UI/AllLevels/Item/Open_Inven.Open_Inven_C" self))
        (`UserWidget.AddToViewport` _returnvalue 0))
      (:`B`
        (`Widget.RemoveFromParent` _returnvalue)))))

(event `Lost item`
  (params (`item name` :type Text))
  ;[1 1 1] 아이템 사용 후 인벤토리에서 그 아이템을 삭제 및 위젯 업데이트
  (for (_array_element _array_index) (`self.Inventory`)
    (if (`KismetTextLibrary.EqualEqual_TextText` (`.Item_Name_6_16B9B9404EF007028E268D95824CE39C` (break `/Game/Blueprints/AllLevels/ItemData` _array_element)) `item name`)
      (`KismetArrayLibrary.Array_Remove` (`self.Inventory`) _array_index)
      (`self.AddItemList`))))

(event `Key|Two`
  (params (Key :type "Key Structure"))
  ;[1 1 1] 아이템 사용 키 바인드
  (:`Pressed`
    (`self.UseItemSelect` 2)))

(event `Key|Three`
  (params (Key :type "Key Structure"))
  ;[1 1 1] 아이템 사용 키 바인드
  (:`Pressed`
    (`self.UseItemSelect` 3)))

(event `Use Item(Searching)`
  ;[1 1 1] Searching 아이템을 사용할 때 발생하는 이벤트
  (if (`KismetMathLibrary.BooleanNOR` (`self.Has_Widget`) (== (`KismetArrayLibrary.Array_Length` (`self.All Player Info`)) 0))
    (bind _returnvalue (`|CreateWidget` "/Game/UI/AllLevels/Item/I_Searching.I_Searching_C"))
    (set `self.Item_Searching WB` _returnvalue)
    (`UserWidget.AddToViewport` (`self.Item_Searching WB`) 0)
    (set `self.bShowMouseCursor` true)
    (`self.MouseTrueMoveStop`)
    (for _array_element (`self.All Player Info`)
      (`/Game/UI/AllLevels/Item/I_Searching.Make Player List` (`self.Item_Searching WB`) _array_element))))

(event `Key|Four`
  (params (Key :type "Key Structure"))
  ;[1 1 1] 아이템 사용 키 바인드
  (:`Pressed`
    (`self.UseItemSelect` 4)))

(event `Select Other Player`
  (params (`Select Index` :type Integer))
  ;[1 1 1] Searching 아이템을 사용할 때 발생하는 이벤트
  (bind _asgameplay_gm (cast `/Game/Blueprints/Gameplay/GameplayGM` (`GameplayStatics.GetGameMode`)))
  (`/Game/Blueprints/Gameplay/GameplayGM.Searching Item Call` _asgameplay_gm self `Select Index`))

(event `Key|Five`
  (params (Key :type "Key Structure"))
  ;[1 1 1] 아이템 사용 키 바인드
  (:`Pressed`
    (`self.UseItemSelect` 5)))

(event `Key|Six`
  (params (Key :type "Key Structure"))
  ;[1 1 1] 아이템 사용 키 바인드
  (:`Pressed`
    (`self.UseItemSelect` 6)))

(event `Search Other Item`
  (params (`Other Inven` :type "Array of /Game/Blueprints/AllLevels/ItemData Structure") (`Other info` :type "/Game/Blueprints/AllLevels/PlayerInfo Structure"))
  (bind _item_searching_wb (`self.Item_Searching WB`))
  ;[1 1 1] Searching 아이템을 사용할 때 발생하는 이벤트
  (set `/Game/UI/AllLevels/Item/I_Searching.Select Player` (`|FormatText` "{name}의 아이템을 \n확인합니다. \n(닫기)" (`.MyPlayerName_2_0D47280F4CABE4536CA4C0A701BBEDF7` (break `/Game/Blueprints/AllLevels/PlayerInfo` `Other info`))) (`self.Item_Searching WB`))
  (for _array_element `Other Inven`
    (`/Game/UI/AllLevels/Item/I_Searching.Make Item List` _item_searching_wb _array_element))
  (`Widget.SetIsEnabled` (`/Game/UI/AllLevels/Item/I_Searching.EXIT_BTN` _item_searching_wb) true))

(fn `Ckeck Item`
  (params (item :type "/Game/Blueprints/AllLevels/ItemData Structure"))
  (returns (ItemtableIndex :type Integer))
  (locals (index :type Integer))
  (bind _returnvalue (`KismetTextLibrary.Conv_TextToString` (`.Item_Name_6_16B9B9404EF007028E268D95824CE39C` (break `/Game/Blueprints/AllLevels/ItemData` item))))
  (if (`KismetStringLibrary.EqualEqual_StrStr` _returnvalue "searching")
    (set `local.index` 3)
    (return (`local.index`))
    (elif (`KismetStringLibrary.EqualEqual_StrStr` _returnvalue "bulletproof")
      (set `local.index` 2)
      (return (`local.index`))
      (elif (`KismetStringLibrary.EqualEqual_StrStr` _returnvalue "gun")
        (set `local.index` 1)
        (return (`local.index`))))))

(fn `LoadGame`
  (bind _returnvalue (`GameplayStatics.LoadGameFromSlot` (`self.PlayerSettingsSave`)))
  (bind _asplayer_save_game (cast `/Game/Blueprints/AllLevels/PlayerSaveGame` _returnvalue))
  (bind (_myplayername _myplayerimage) (break `/Game/Blueprints/AllLevels/PlayerInfo` (`/Game/Blueprints/AllLevels/PlayerSaveGame.S_PlayerInfo` _asplayer_save_game)))
  (setmembers `/Game/Blueprints/AllLevels/PlayerInfo` :`StructRef` (`self.Player Setting`) :`MyPlayerName` _myplayername :`MyPlayerImage` _myplayerimage))

(fn `UserConstructionScript`)