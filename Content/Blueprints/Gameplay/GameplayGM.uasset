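; Server game mode for a multiplayer match with assigned jobs, missions and player voting.
; It takes jobs from GameInfoInstance, assigns them as controllers arrive, spawns pawns at random PlayerStarts and relays mission updates and item searches.
; Looping timers push countdowns to each GameplayPC, while votes are tallied with ties sent to a revote.
; It also server-travels to a climbing minigame; the converted game time is unused, with SettingTime fixed instead.
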(event `GetGameSettings`
  ;[1 1 1] 게임 인스턴스에 있는 정보 넘겨받음
  (if (`KismetSystemLibrary.IsServer`)
    (bind _asgame_info_instance (cast `/Game/Blueprints/AllLevels/GameInfoInstance` (`GameplayStatics.GetGameInstance`)))
    (set `self.AllplayerJob` (`/Game/Blueprints/AllLevels/GameInfoInstance.JobArray` _asgame_info_instance))
    (`self.TextToFloat` (`/Game/Blueprints/AllLevels/GameInfoInstance.Game TIme` _asgame_info_instance))
    (set `self.SettingTime` 5.0)))

(event `self.K2_OnSwapPlayerControllers`
  (params (OldPC :type "PlayerController Object Reference") (NewPC :type "PlayerController Object Reference"))
  ;[1 1 1] 동일
  (`self.GetGameSettings`)
  (`/Engine/EditorBlueprintResources/ActorMacros.Switch Has Authority`
    (:`Authority`
      (bind _returnvalue (`KismetArrayLibrary.Array_Add` (`self.AllPlayerControllers`) NewPC))
      (bind _outactors (`GameplayStatics.GetAllActorsOfClass` "/Script/Engine.PlayerStart"))
      (set `self.Respawn Point` _outactors)
      (bind _asgameplay_pc (cast `/Game/Blueprints/Gameplay/GameplayPC` NewPC))
      (bind _structout (setmembers `/Game/Blueprints/AllLevels/PlayerInfo` :`StructRef` (`/Game/Blueprints/Gameplay/GameplayPC.Player Setting` _asgameplay_pc) :`MyPlayerJob` (`|GetArrayItem` (`self.AllplayerJob`) _returnvalue)))
      (`/Game/Blueprints/Gameplay/GameplayPC.PlayStart` _asgameplay_pc _structout))))

(event `CheckAllSpawn2`
  ;[1 1 1] 모든 플레이어가 스폰되면 알리고 남은 투표시간을 시작함
  (if (== (`KismetArrayLibrary.Array_Length` (`self.AllPlayerControllers`)) (`KismetArrayLibrary.Array_Length` (`self.AllplayerJob`)))
    (set `self.AllUserSpawn?` true)
    (`self.GetAllPlayerInfo`)
    (`self.VoteTime`)
    (else
      (set `self.AllUserSpawn?` false))))

(event `RespawnPlayer`
  (params (`Player Controller` :type "PlayerController Object Reference"))
  (bind _returnvalue (`Controller.K2_GetPawn` `Player Controller`))
  (bind _respawn_point (`self.Respawn Point`))
  ;[1 1 1] 캐릭터들의 플레이어 컨트롤러를 받아서 스폰함
  (`KismetSystemLibrary.Delay` 0.5)
  (`/Engine/EditorBlueprintResources/StandardMacros.IsValid` _returnvalue
    (:`Is Valid`
      (`self.K2_DestroyActor` _returnvalue))
    (:`Is Not Valid`
      _))
  (bind _returnvalue_2 (`|SpawnActorFromClass` "/Game/Blueprints/Characters/0_Base.0_Base_C" (`self.GetTransform` (`|GetArrayItem` _respawn_point (`KismetMathLibrary.RandomInteger` (`KismetArrayLibrary.Array_Length` _respawn_point)))) "Undefined" "OverrideRootScale" null (`/Game/Blueprints/Gameplay/GameplayPC.avatars` (cast `/Game/Blueprints/Gameplay/GameplayPC` `Player Controller` :!pure true)) null))
  (`self.RespawnPlayer` null)
  (`Controller.Possess` `Player Controller` _returnvalue_2))

(event `MissionUpdate`
  ;[1 1 1] 플레이어 직업과 미션 진행상황을 업데이트
  (for _array_element (`self.AllPlayerControllers`)
    (bind _asgameplay_pc (cast `/Game/Blueprints/Gameplay/GameplayPC` _array_element))
    (set `/Game/Blueprints/Gameplay/GameplayPC.MissionOfPlayer` (`self.Mission`) _asgameplay_pc)
    (`/Game/Blueprints/Gameplay/GameplayPC.UpdateMission` _asgameplay_pc)))

(event `self.K2_OnLogout`
  (params (ExitingController :type "Controller Object Reference"))
  ;[1 1 1] 로그아웃하면 세션 종료
  (bind _asgameplay_pc (cast `/Game/Blueprints/Gameplay/GameplayPC` ExitingController))
  (`/Game/Blueprints/AllLevels/GameInfoInstance.DestroySessionCaller` (cast `/Game/Blueprints/AllLevels/GameInfoInstance` (`GameplayStatics.GetGameInstance`) :!pure true) _asgameplay_pc))

(event `GetAllPlayerInfo`
  ;[1 1 1] 투표에 필요한 배열 정리 및 초기화
  (`KismetArrayLibrary.Array_Clear` (`self.AllPlayerInfo`))
  (`KismetArrayLibrary.Array_Clear` (`self.PlayerVote`))
  (for _array_element (`self.AllPlayerControllers`)
    (bind _asgameplay_pc (cast `/Game/Blueprints/Gameplay/GameplayPC` _array_element))
    (`KismetArrayLibrary.Array_Add` (`self.AllPlayerInfo`) (`/Game/Blueprints/Gameplay/GameplayPC.Player Setting` _asgameplay_pc))
    (`KismetArrayLibrary.Array_Add` (`self.PlayerVote`))
    (set `/Game/Blueprints/Gameplay/GameplayPC.Voted` false _asgameplay_pc)))

(event `DoMission`
  ;[1 1 1] 미션이 진행되면 발생
  (setmembers `/Game/Blueprints/AllLevels/Mission` :`StructRef` (`self.Mission`) :`Mission_1` true)
  (`self.MissionUpdate`))

(event `VoteResult`
  (bind _playervote (`self.PlayerVote`))
  (bind (_indexofmaxvalue _maxvalue) (`KismetMathLibrary.MaxOfIntArray` _playervote))
  ;[1 1 1] 뽑힌 플레이어를 모든 플레이어에게 알리고 그 플레이어 정보를 넘김
  (bind (_newparam _defultindex) (`self.FindSameMaxValue` _playervote _maxvalue))
  (if _newparam
    (`self.ReVote` _defultindex)
    (else
      (for _array_element (`self.AllPlayerControllers`)
        (bind _asgameplay_pc (cast `/Game/Blueprints/Gameplay/GameplayPC` _array_element))
        (`/Game/Blueprints/Gameplay/GameplayPC.InformPickedPlayer` _asgameplay_pc (`|GetArrayItem` (`self.AllPlayerInfo`) _indexofmaxvalue))))))

(event `CheckVoteComplete`
  ;[1 1 1] 각 플레이어가 모두 투표를 완료했는지 확인하고 완료했다면 투표 결과 집계
  (set `self.temp_voted` true)
  (for _array_element (`self.AllPlayerControllers`)
    (bind _asgameplay_pc (cast `/Game/Blueprints/Gameplay/GameplayPC` _array_element))
    (set `self.temp_voted` (and (`/Game/Blueprints/Gameplay/GameplayPC.Voted` _asgameplay_pc) (`self.temp_voted`))))
  (if (`self.temp_voted`)
    (`self.VoteResult`)))

(event `VoteTime`
  ;[1 1 1] 1초가 지날 때 마다 타이머를 각 유저에게 업데이트
  (set `self.VoteRemainingTime` (`self.SettingTime`))
  (bind _returnvalue (`KismetSystemLibrary.K2_SetTimerDelegate` (delegate `TimeSee`) 1.0 true))
  (set `self.VoteTimer` _returnvalue))

(event `TimeSee`
  ;[1 1 1] 1초가 지날 때 마다 타이머를 각 유저에게 업데이트
  (set `self.VoteRemainingTime` (- (`self.VoteRemainingTime`) 1.0))
  (for _array_element (`self.AllPlayerControllers`)
    (bind _asgameplay_pc (cast `/Game/Blueprints/Gameplay/GameplayPC` _array_element))
    (`/Game/Blueprints/Gameplay/GameplayPC.UpdateTimer` _asgameplay_pc (`self.VoteRemainingTime`))))

(event `VoteStart`
  ;[1 1 1] 투표시간이 되면 시간을 멈추고 투표창 열라고 통보
  (`KismetSystemLibrary.K2_ClearAndInvalidateTimerHandle` (`self.VoteTimer`))
  (`self.GetAllPlayerInfo`)
  (for _array_element (`self.AllPlayerControllers`)
    (bind _asgameplay_pc (cast `/Game/Blueprints/Gameplay/GameplayPC` _array_element))
    (`/Game/Blueprints/Gameplay/GameplayPC.Makevotewindow` _asgameplay_pc (`self.AllPlayerInfo`)))
  (`self.CountVoteTime`))

(event `ReVote`
  (params (Indexs :type "Array of Integer"))
  ;[1 1 1] 뽑힌 사람이 다수일 경우 다시 투표함
  (`KismetArrayLibrary.Array_Clear` (`self.NewVar_0`))
  (for _array_element Indexs
    (`KismetArrayLibrary.Array_Add` (`self.NewVar_0`) (`|GetArrayItem` (`self.AllPlayerInfo`) _array_element)))
  (for _array_element_2 (`self.AllPlayerControllers`)
    (bind _asgameplay_pc (cast `/Game/Blueprints/Gameplay/GameplayPC` _array_element_2))
    (set `/Game/Blueprints/Gameplay/GameplayPC.Voted` false _asgameplay_pc)
    (`/Game/Blueprints/Gameplay/GameplayPC.ReadyRevote` _asgameplay_pc (`self.NewVar_0`))
    (`KismetSystemLibrary.Delay` 2.0)
    (`self.CountVoteTime`)))

(event `CountVoteTime`
  ;[1 1 1] 투표 중 시간을 제한
  (set `self.VoteRemaingTime2` 3.0)
  (bind _returnvalue (`KismetSystemLibrary.K2_SetTimerDelegate` (delegate `TimeSee2`) 1.0 true)))

(event `TimeSee2`
  ;[1 1 1] 투표 중 시간을 제한
  (bind _output_get (set `self.VoteRemaingTime2` (- (`self.VoteRemaingTime2`) 1.0)))
  (if (<= _output_get -2.0)
    (`KismetSystemLibrary.K2_ClearAndInvalidateTimerHandle` (stale `CountVoteTime` _returnvalue))
    (else
      (for _array_element (`self.AllPlayerControllers`)
        (bind _asgameplay_pc (cast `/Game/Blueprints/Gameplay/GameplayPC` _array_element))
        (`/Game/Blueprints/Gameplay/GameplayPC.UpdateTimer2` _asgameplay_pc (`self.VoteRemaingTime2`))))))

(event `MiniGame`
  ;[1 1 1] 미니게임 스타드 이벤트
  (set `/Game/Blueprints/AllLevels/GameInfoInstance.SaveRemainingTime` (`self.VoteRemainingTime`) (cast `/Game/Blueprints/AllLevels/GameInfoInstance` (`GameplayStatics.GetGameInstance`) :!pure true))
  (for _array_element (`self.AllPlayerControllers`)
    (bind _asgameplay_pc (cast `/Game/Blueprints/Gameplay/GameplayPC` _array_element))
    (`/Game/Blueprints/Gameplay/GameplayPC.ShowLoadingScreen` _asgameplay_pc))
  (`KismetSystemLibrary.ExecuteConsoleCommand` "servertravel Minigame_Climb" (`GameplayStatics.GetPlayerController` 0)))

(event `Searching Item Call`
  (params (`Call PC` :type "PlayerController Object Reference") (`Called Index` :type Integer))
  (bind _asgameplay_pc (cast `/Game/Blueprints/Gameplay/GameplayPC` (`|GetArrayItem` (`self.AllPlayerControllers`) `Called Index`) :!pure true))
  ;[1 1 1] 플레이어가 요청한 Searching 아이템 사용을 응답하고 대상이 된 플레이어의 정보를 반환
  (`/Game/Blueprints/Gameplay/GameplayPC.Search Other Item` (cast `/Game/Blueprints/Gameplay/GameplayPC` `Call PC` :!pure true) (`/Game/Blueprints/Gameplay/GameplayPC.Inventory` _asgameplay_pc) (`/Game/Blueprints/Gameplay/GameplayPC.Player Setting` _asgameplay_pc)))

(fn `FindSameMaxValue`
  (params (Player :type "Array of Integer") (Max :type Integer))
  (returns (NewParam :type Boolean) (DefultIndex :type "Array of Integer"))
  (locals (IsSameMaxValue :type Boolean) (SameIndex :type "Array of Integer"))
  (for (_array_element _array_index) Player
    (if (== _array_element Max)
      (`KismetArrayLibrary.Array_Add` (`local.SameIndex`) _array_index)))
  (if (> (`KismetArrayLibrary.Array_Length` (`local.SameIndex`)) 1)
    (set `local.IsSameMaxValue` true)
    (else
      (set `local.IsSameMaxValue` false)))
  (return (`local.IsSameMaxValue`) (`local.SameIndex`)))

(fn `TextToFloat`
  (params (Input :type Text))
  (returns (Output :type "Float (double-precision)"))
  (locals (`10:00` :type Text :default "NSLOCTEXT(\"\", \"D94D2D2D4DB3299FB8772D8988B015E1\", \"10:00\")") (`15:00` :type Text :default "NSLOCTEXT(\"\", \"3788D6FD4C344317816E208A53B7C0F1\", \"15:00\")") (`20:00` :type Text :default "NSLOCTEXT(\"\", \"1275140E4C90EFF8116255A911937198\", \"20:00\")") (`25:00` :type Text :default "NSLOCTEXT(\"\", \"22945C46407CE6A7E58E42B4B76A41A8\", \"25:00\")") (TempFloat :type "Float (double-precision)"))
  (if (`KismetTextLibrary.EqualEqual_TextText` Input (`local.10:00`))
    (set `local.TempFloat` 600.0)
    (elif (`KismetTextLibrary.EqualEqual_TextText` Input (`local.15:00`))
      (set `local.TempFloat` 900.0)
      (elif (`KismetTextLibrary.EqualEqual_TextText` Input (`local.20:00`))
        (set `local.TempFloat` 1200.0)
        (elif (`KismetTextLibrary.EqualEqual_TextText` Input (`local.25:00`))
          (set `local.TempFloat` 1500.0)
          (else
            (set `local.TempFloat` 900.0))))))
  (return (`local.TempFloat`)))

(fn `UserConstructionScript`)