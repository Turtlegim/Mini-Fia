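; Light1 is an actor that travels along the spline of a referenced track actor, TrackRef1.
; On BeginPlay it derives the timeline play rate from a duration, applies a start offset, then plays the timeline.
; Each update maps the timeline alpha to spline distance and sets the actor's location and rotation from that point.
; The spline is sampled in local space, and those values are applied directly as the actor's world transform.
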(event `self.ReceiveBeginPlay`
  (bind _returnvalue (`KismetMathLibrary.Lerp` 0.0 (`SplineComponent.GetSplineLength` (`/Game/Blueprints/Actor/Track1.Spline1` (`self.TrackRef1`))) (`self.Alpha1`)))
  (`TimelineComponent.SetPlayRate` (`self.타임라인_1`) (/ 1.0 (`self.Duration1`)))
  (`TimelineComponent.SetNewTime` (`self.타임라인_1`) (`self.StartOffset1`))
  (bind (_direction `_새_트랙_0`) (`Timeline|타임라인_1`)
    (:`Update`
      (set `self.Alpha1` `_새_트랙_0`)
      (`self.K2_SetActorLocationAndRotation` (`SplineComponent.GetLocationAtDistanceAlongSpline` (`/Game/Blueprints/Actor/Track1.Spline1` (`self.TrackRef1`)) _returnvalue "Local") (`SplineComponent.GetRotationAtDistanceAlongSpline` (`/Game/Blueprints/Actor/Track1.Spline1` (`self.TrackRef1`)) _returnvalue "Local")))))

(fn `UserConstructionScript`)