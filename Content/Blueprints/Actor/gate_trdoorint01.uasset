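; Two-panel sliding gate actor with custom events to open and close it and to reposition a separate Block01 component.
; One timeline, played forward or reversed, drives both meshes, with the second mirrored along Y from a fixed offset.
; Separate open and close block events snap Block01 vertically between raised and lowered positions without sweep, independently of the door animation.
; A second timeline is present but unused.
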(event `open01`
  (bind (_direction `_새_트랙_0`) (`Timeline|타임라인_0` :!label _label)
    (:`Update`
      (`SceneComponent.K2_SetRelativeLocation` (`self.StaticMesh`) `_새_트랙_0` false false)
      (`SceneComponent.K2_SetRelativeLocation` (`self.StaticMesh1`) (+ (0.0 480.0 0.0) (* (0.0 -1.0 0.0) `_새_트랙_0`)) false false))))

(event `close01`
  (goto _label :!via `Reverse`))

(event `open_block01`
  (`SceneComponent.K2_SetRelativeLocation` (`self.block01`) (0.0 0.0 1000.0) false false))

(event `close_block01`
  (`SceneComponent.K2_SetRelativeLocation` (`self.block01`) (0.0 0.0 -1000.0) false false))

(fn `UserConstructionScript`)