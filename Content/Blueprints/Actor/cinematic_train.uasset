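; Cinematic train actor that rides along the spline of a referenced track, starting on BeginPlay when its Activekart flag is set.
; MoveKart scales the KartMover timeline's play rate by the inverse of Duration and starts it from KartStartOffset.
; Each timeline update maps Alpha to a distance along the spline and sets the actor's world location and rotation to match.
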(event `self.ReceiveBeginPlay`
  (if (`self.activekart`)
    (`self.MoveKart`)))

(event `MoveKart`
  (bind _returnvalue (`KismetMathLibrary.Lerp` 0.0 (`SplineComponent.GetSplineLength` (`/Game/Blueprints/Actor/Track.Spline` (`self.TrackRef`))) (`self.Alpha`)))
  (`TimelineComponent.SetPlayRate` (`self.KartMover`) (/ 1.0 (`self.Duration`)))
  (`TimelineComponent.SetNewTime` (`self.KartMover`) (`self.KartStartOffset`))
  (bind (_direction _alpha) (`Timeline|KartMover`)
    (:`Update`
      (set `self.Alpha` _alpha)
      (`self.K2_SetActorLocationAndRotation` (`SplineComponent.GetLocationAtDistanceAlongSpline` (`/Game/Blueprints/Actor/Track.Spline` (`self.TrackRef`)) _returnvalue "World") (`SplineComponent.GetRotationAtDistanceAlongSpline` (`/Game/Blueprints/Actor/Track.Spline` (`self.TrackRef`)) _returnvalue "World")))))

(fn `UserConstructionScript`)